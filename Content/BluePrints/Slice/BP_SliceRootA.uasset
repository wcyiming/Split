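; BP_SliceRootA is a child Blueprint that limits its SceneCap scene capture to a tagged subset of the level's actors.
; On BeginPlay, after the parent's logic, it switches the capture to show-only mode and clears the show-only components.
; It then merges actors tagged "Need" and "ActorA" into the show-only actor list.
; Tick and construction only call the parent.
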(event `self.ReceiveBeginPlay`
  (bind _scenecap (`self.SceneCap`))
  (`parent.ReceiveBeginPlay`)
  (set `SceneCaptureComponent.PrimitiveRenderMode` "PRM_UseShowOnlyList" _scenecap)
  (`SceneCaptureComponent.ClearShowOnlyComponents` _scenecap)
  (bind _outactors (`GameplayStatics.GetAllActorsWithTag` "Need"))
  (bind _output_get (set `self.ActorArray` _outactors))
  (bind _outactors_2 (`GameplayStatics.GetAllActorsWithTag` "ActorA"))
  (`KismetArrayLibrary.Array_Append` _output_get _outactors_2)
  (set `SceneCaptureComponent.ShowOnlyActors` (`self.ActorArray`) _scenecap))

(event `self.ReceiveTick`
  (params (DeltaSeconds :type "Float (single-precision)"))
  (`parent.ReceiveTick` DeltaSeconds))

(fn `UserConstructionScript`
  (`parent.UserConstructionScript`))